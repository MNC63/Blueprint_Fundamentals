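; BP_Variables is a Blueprint that demonstrates setting and printing variables when play begins.
; On BeginPlay it prints FirstVar, sets it to a new value and prints it again.
; It then reassigns SecondVar through a literal, a product with JumpHieght and a nested sum, printing each step in colored on-screen text, some with longer durations.
; The construction script is empty.
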(event `self.ReceiveBeginPlay`
  (`KismetSystemLibrary.PrintString` (`KismetStringLibrary.Conv_IntToString` (`self.FirstVar`)))
  (set `self.FirstVar` 2)
  (`KismetSystemLibrary.PrintString` (`KismetStringLibrary.Conv_IntToString` (`self.FirstVar`)))
  (`KismetSystemLibrary.PrintString` (`KismetStringLibrary.Conv_DoubleToString` (`self.SecondVar`)) true true (struct :`R` 0.926805 :`G` 1.0 :`B` 0.2177 :`A` 1.0))
  (set `self.SecondVar` 4.5)
  (`KismetSystemLibrary.PrintString` (`KismetStringLibrary.Conv_DoubleToString` (`self.SecondVar`)) true true (struct :`R` 1.0 :`G` 0.993957 :`B` 0.220934 :`A` 1.0) 4.0)
  (bind _output_get (set `self.SecondVar` (* 5.5 (`self.JumpHieght`))))
  (`KismetSystemLibrary.PrintString` (`KismetStringLibrary.Conv_DoubleToString` (`self.SecondVar`)) true true (struct :`R` 1.0 :`G` 0.183489 :`B` 0.187308 :`A` 1.0) 6.0)
  (set `self.SecondVar` (+ (`self.JumpHieght`) (+ _output_get (`self.JumpHieght`))))
  (`KismetSystemLibrary.PrintString` (`KismetStringLibrary.Conv_DoubleToString` (`self.SecondVar`)) true true (struct :`R` 0.958608 :`G` 0.3665 :`B` 1.0 :`A` 1.0) 6.0))

(fn `UserConstructionScript`)