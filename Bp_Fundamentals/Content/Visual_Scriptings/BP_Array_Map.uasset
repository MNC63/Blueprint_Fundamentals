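; BP_Array_Map is a scripting demo of array and map operations that prints results to the screen.
; On BeginPlay, after a short delay, it prints a value looked up by key in the Weapon map, then adds an entry and prints that in another color.
; A disconnected Fruits array example covers reading by index, setting an element and replacing the whole array, but never runs.
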(event `self.ReceiveBeginPlay`
  (`KismetSystemLibrary.Delay` 4.0)
  (`KismetSystemLibrary.PrintString` (`BlueprintMapLibrary.Map_Find` (`self.Weapon`) 4) true true (struct :`R` 1.0 :`G` 0.370517 :`B` 0.30068 :`A` 1.0))
  (`BlueprintMapLibrary.Map_Add` (`self.Weapon`) 8 "Odin")
  (`KismetSystemLibrary.PrintString` (`BlueprintMapLibrary.Map_Find` (`self.Weapon`) 8) true true (struct :`R` 0.886446 :`G` 1.0 :`B` 0.055208 :`A` 1.0)))

(fn `UserConstructionScript`)