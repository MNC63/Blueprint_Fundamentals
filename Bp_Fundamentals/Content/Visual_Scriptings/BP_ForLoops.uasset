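; Loop demonstration Blueprint that rescales house actors in the level shortly after play begins.
; After a delay, BeginPlay calls HouseScales, which iterates all BP_HouseTemplate actors and sets their world scale, giving odd-indexed houses a larger multiple of the target.
; An unused PrintFruit event shows an index loop pluralizing Fruit array entries, then a for-each loop printing each with its index and a finish message.
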(event `self.ReceiveBeginPlay`
  (`KismetSystemLibrary.Delay` 2.0)
  (`self.House Scales` (2.0 2.0 2.0)))

(event `House Scales`
  (params (`Target Scale` :type "Vector Structure"))
  (bind _outactors (`GameplayStatics.GetAllActorsOfClass` "/Game/Visual_Scriptings/BP_HouseTemplate.BP_HouseTemplate_C"))
  (for (_array_element _array_index) _outactors
    (if (== (mod _array_index 2) 0)
      (bind _rootcomponent (`Actor.RootComponent` _array_element))
      (`SceneComponent.SetWorldScale3D` _rootcomponent `Target Scale`)
      (else
        (`SceneComponent.SetWorldScale3D` _rootcomponent (* `Target Scale` 2.5))))))

(event `PrintFruit`
  (bind _fruit (`self.Fruit`))
  (for _index (range (`KismetArrayLibrary.Array_Length` (`self.Fruit`)))
    (`KismetArrayLibrary.Array_Set` _fruit _index (`KismetStringLibrary.Concat_StrStr` (`|GetArrayItem` _fruit _index) "s")))
  (for (_array_element _array_index) (`self.Fruit`)
    ; Loop Body
    (`KismetSystemLibrary.PrintString` (`KismetStringLibrary.Concat_StrStr` _array_element ":" (`KismetStringLibrary.Conv_IntToString` _array_index)) true true (struct :`R` 1.0 :`G` 0.106856 :`B` 0.122136 :`A` 1.0) 12.0))
  ; Finished
  (`KismetSystemLibrary.PrintString` "Finished" true true (struct :`R` 0.024762 :`G` 0.223958 :`B` 0.006309 :`A` 1.0) 12.0))

(fn `UserConstructionScript`)