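; BP_House is an actor that builds a simple house from primitive meshes at runtime.
; After a delay on BeginPlay, it adds static mesh components for a cube foundation, four cube walls and a two-ramp roof, each positioned and scaled relative to the actor.
; It then sets the root's world scale three times at timed intervals, each from the same multiple of ScaleVector, which the graph never updates.
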(event `self.ReceiveBeginPlay`
  (`KismetSystemLibrary.PrintString` "Start Construction")
  (`KismetSystemLibrary.Delay` 3.0)
  ; Foundation
  (bind _returnvalue (`AddComponent|NODE_AddStaticMeshComponent-0`))
  (`StaticMeshComponent.SetStaticMesh` _returnvalue "/Engine/EngineMeshes/Cube.Cube")
  (`SceneComponent.K2_SetRelativeLocation` _returnvalue (0.0 0.0 5.0) false false)
  (`SceneComponent.SetRelativeScale3D` _returnvalue (1.0 1.0 0.1))
  ; Walls
  (bind _returnvalue_2 (`AddComponent|NODE_AddStaticMeshComponent-1` :`RelativeTransform` (`KismetMathLibrary.MakeTransform` (-70.0 -1.0 39.0) (struct :`Yaw` 90.0) (0.75 0.05 0.6))))
  (`StaticMeshComponent.SetStaticMesh` _returnvalue_2 "/Engine/EngineMeshes/Cube.Cube")
  (bind _returnvalue_3 (`AddComponent|NODE_AddStaticMeshComponent-2` :`RelativeTransform` (`KismetMathLibrary.MakeTransform` (70.0 -1.0 39.0) (struct :`Yaw` 90.0) (0.75 0.05 0.6))))
  (`StaticMeshComponent.SetStaticMesh` _returnvalue_3 "/Engine/EngineMeshes/Cube.Cube")
  (bind _returnvalue_4 (`AddComponent|NODE_AddStaticMeshComponent-3` :`RelativeTransform` (`KismetMathLibrary.MakeTransform` (0.0 70.0 39.0) (struct) (0.75 0.05 0.6))))
  (`StaticMeshComponent.SetStaticMesh` _returnvalue_4 "/Engine/EngineMeshes/Cube.Cube")
  (bind _returnvalue_5 (`AddComponent|NODE_AddStaticMeshComponent-4` :`RelativeTransform` (`KismetMathLibrary.MakeTransform` (0.0 -70.0 39.0) (struct) (0.75 0.05 0.6))))
  (`StaticMeshComponent.SetStaticMesh` _returnvalue_5 "/Engine/EngineMeshes/Cube.Cube")
  ; Roof
  (bind _returnvalue_6 (`AddComponent|NODE_AddStaticMeshComponent-5` :`RelativeTransform` (`KismetMathLibrary.MakeTransform` (150.0 0.0 110.0) (struct :`Yaw` 180.0) (3.0 1.5 1.0))))
  (`StaticMeshComponent.SetStaticMesh` _returnvalue_6 "/Game/LevelPrototyping/Meshes/SM_Ramp.SM_Ramp")
  (bind _returnvalue_7 (`AddComponent|NODE_AddStaticMeshComponent-6` :`RelativeTransform` (`KismetMathLibrary.MakeTransform` (-150.0 0.0 110.0) (struct) (3.0 1.5 1.0))))
  (`StaticMeshComponent.SetStaticMesh` _returnvalue_7 "/Game/LevelPrototyping/Meshes/SM_Ramp.SM_Ramp")
  (`KismetSystemLibrary.Delay` 2.0)
  (`SceneComponent.SetWorldScale3D` (`self.DefaultSceneRoot`) (* (`self.ScaleVector`) 2.5))
  (`KismetSystemLibrary.Delay` 2.0)
  (`SceneComponent.SetWorldScale3D` (`self.DefaultSceneRoot`) (* (`self.ScaleVector`) 2.5))
  (`KismetSystemLibrary.Delay` 2.0)
  (`SceneComponent.SetWorldScale3D` (`self.DefaultSceneRoot`) (* (`self.ScaleVector`) 2.5)))

(fn `UserConstructionScript`)